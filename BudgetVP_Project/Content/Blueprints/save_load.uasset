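; Actor that demonstrates asynchronously saving and loading a calibration point through a PositionData save game, apparently as a template with placeholder logic.
; BeginPlay adds an Enhanced Input context and loads the "CalibrationValues" slot, printing the point from the immediate then pin rather than on completion.
; The save_data input saves a new PositionData, with CalibrationPoint left unfilled, to that object's own slot and prints success or failure.
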(event `self.ReceiveBeginPlay`
  ;[1 1 1] get player controller for input
  (bind _asplayer_controller (cast `PlayerController` (`Pawn.GetController` (`GameplayStatics.GetPlayerPawn` 0))))
  (`EnhancedInputSubsystemInterface.AddMappingContext` (pcsubsystem `EnhancedInputLocalPlayerSubsystem` _asplayer_controller) "/Game/sava_data_Context.sava_data_Context" 0 (struct))
  ;[1 1 1] Do Something here to load the value you Saved
  (bind _savegame (`AsyncActionHandleSaveGame.AsyncLoadGameFromSlot` "CalibrationValues")
    (:`then`
      (bind _asposition_data (cast `/Game/Blueprints/PositionData` _savegame))
      (bind _output_get (set `self.LoadedValue` (`/Game/Blueprints/PositionData.Calibration_Point` _asposition_data)))
      (`KismetSystemLibrary.PrintString` (`KismetStringLibrary.Concat_StrStr` "Loaded Point: " (`KismetStringLibrary.Conv_VectorToString` _output_get))))))

(event `EnhancedInput|/Game/save_data`
  (params (ActionValue :type Boolean) (ElapsedSeconds :type "Float (double-precision)") (TriggeredSeconds :type "Float (double-precision)") (InputAction :type "InputAction Object Reference" :default "/Game/save_data.save_data"))
  (:`Started`
    ;[1 1 1] do something here to save the value on button press
    (bind _returnvalue (`GameplayStatics.CreateSaveGameObject` "/Game/Blueprints/PositionData.PositionData_C"))
    (set `/Game/Blueprints/PositionData.Calibration_Point` (0.0 0.0 0.0) _returnvalue)
    (bind (_savegame _bsuccess) (`AsyncActionHandleSaveGame.AsyncSaveGameToSlot` _returnvalue (`/Game/Blueprints/PositionData.SaveSlotName` _returnvalue) (`/Game/Blueprints/PositionData.UserIndex` _returnvalue))
      (:`Completed`
        (if _bsuccess
          (`KismetSystemLibrary.PrintString` "Saved!")
          (else
            (`KismetSystemLibrary.PrintString` "Failed.")))))))

(fn `UserConstructionScript`)
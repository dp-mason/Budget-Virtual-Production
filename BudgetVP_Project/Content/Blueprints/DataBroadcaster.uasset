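; DataBroadcaster is an actor that broadcasts MIDI input and master-track audio analysis through event dispatchers.
; It binds every MIDI device on BeginPlay, with manual (M) and periodic (N-toggled) re-initialization as a workaround for dropouts.
; Space and arrow keys control playback and seeking.
; Playback updates sample loudness analyzers, then broadcast them with spectrum analyzers and a timestamp offset by XRDelay to match delayed video.
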(event `self.ReceiveTick`
  (params (DeltaSeconds :type "Float (single-precision)"))
  (bind _debugmidi (`self.debugMIDI`))
  (bind _debugmidi_2 (`self.debugMIDI`))
  (bind _debugmidi_3 (`self.debugMIDI`))
  ;[1 0 0] JANKY FIX - the MIDI input system breaks every once in a while. Reinitializing fixes the issue, but this is a really terrible solution, unreliable.
  (if (and (== (mod (`KismetMathLibrary.FTrunc` (`KismetSystemLibrary.GetGameTimeInSeconds`)) (`self.reInitRate_JankFix`)) 0) (`self.autoReinitMidi`))
    ;[0 1 0.817] Init MIDI devices
    (`KismetArrayLibrary.Array_Clear` (`self.midiDevices`) :!label _label)
    (bind _outmididevices (`MIDIDeviceManager.FindMIDIDevices`))
    (bind _output_get (set `self.midiDevices` _outmididevices))
    (if (`self.debugMIDI`)
      (for (_array_element _array_index) _output_get
        (bind (_deviceid _devicename) (break `FoundMIDIDevice` _array_element))
        (`KismetSystemLibrary.PrintString` (`KismetStringLibrary.Concat_StrStr` "MIDI Device " (`KismetStringLibrary.Conv_IntToString` _array_index) ": " (`KismetStringLibrary.Conv_IntToString` _deviceid) " " _devicename) _debugmidi_3 _debugmidi_3 (struct :`G` 0.66 :`B` 1.0 :`A` 1.0) 1.0 "device")))
    (for _array_element_2 _output_get
      (bind (_deviceid_2 _devicename_2) (break `FoundMIDIDevice` _array_element_2))
      (bind _returnvalue (`MIDIDeviceManager.CreateMIDIDeviceController` _deviceid_2 512))
      (`/Engine/EditorBlueprintResources/StandardMacros.IsValid` _returnvalue
        (:`Is Valid`
          (add `MIDIDeviceController.OnMIDIEvent` _returnvalue (delegate `MIDI Event`))
          (bind _returnvalue_2 (`KismetStringLibrary.ToLower` _devicename_2))
          (`KismetSystemLibrary.PrintString` (`KismetStringLibrary.Concat_StrStr` "Initialized  " _returnvalue_2) _debugmidi _debugmidi (struct :`G` 1.0 :`B` 0.156256 :`A` 1.0) 12.0 "device_2"))
        (:`Is Not Valid`
          (`KismetSystemLibrary.PrintString` (`KismetStringLibrary.Concat_StrStr` "MIDI INIT FAILED FOR " _returnvalue_2) _debugmidi_2 _debugmidi_2 (struct :`R` 1.0 :`B` 0.061703 :`A` 1.0) 20.0 "failure_midi"))))))

(event `Key|N`
  (params (Key :type "Key Structure"))
  (:`Pressed`
    (bind _isa (`/Engine/EditorBlueprintResources/StandardMacros.FlipFlop`)
      (:`A`
        _)
      (:`B`
        _))
    (set `self.autoReinitMidi` _isa)))

(event `Key|M`
  (params (Key :type "Key Structure"))
  ;[1 1 1] Sometimes MIDI gets disconnected, press M to re-initialize
  (:`Pressed`
    (goto _label)))

(event `MIDI Event`
  (params (MIDIDeviceController :type "MIDIDeviceController Object Reference") (Timestamp :type Integer) (EventType :type "EMIDIEventType Enum" :default "Unknown") (Channel :type Integer) (ControlID :type Integer) (Velocity :type Integer) (RawEventType :type Integer))
  (bind _debugmidi (`self.debugMIDI`))
  (bind _devicename (`MIDIDeviceController.DeviceName` MIDIDeviceController))
  ;[0 1 0.8548] Comment
  (if (`self.debugMIDI`)
    (`KismetSystemLibrary.PrintString` (`KismetStringLibrary.Concat_StrStr` "Device " _devicename " Produced Control: " (`KismetStringLibrary.Conv_IntToString` RawEventType) " with ID: " (`KismetStringLibrary.Conv_IntToString` ControlID) " and Velocity: " (`KismetStringLibrary.Conv_IntToString` Velocity) "/127" "CHANNEL: " (`KismetStringLibrary.Conv_IntToString` Channel)) _debugmidi _debugmidi (struct :`G` 0.66 :`B` 1.0 :`A` 1.0) 2.0 "recentMidiEvent"))
  (`self.MIDI_InputEvent` _devicename Timestamp Channel ControlID Velocity RawEventType))

(event `self.ReceiveBeginPlay`
  (bind _debugaudio (`self.debugAudio`))
  (bind _masteraudiosource (`self.MasterAudioSource`))
  (`|ExecutionSequence`
    (:`then_0`
      (goto _label))
    (:`then_1`
      ;[0.648 0 1] Audio, Enable Keyboard Input For PLay/Pause
      (`KismetSystemLibrary.PrintString` "Configuring Audio" _debugaudio _debugaudio)
      (`self.EnableInput` (`GameplayStatics.GetPlayerController` 0))
      ;[0.6439 0 1] Audio
      (`AudioComponent.SetSound` (`self.Audio`) _masteraudiosource)
      (set `self.audioDurationFraction` (/ 1.0 (`SoundBase.Duration` _masteraudiosource)))
      ;[0.6439 0 1] Audio
      (add `AudioComponent.OnAudioPlaybackPercent` (`self.Audio`) (delegate `UpdateSongElapsed`)))))

(event `Key|Right`
  (params (Key :type "Key Structure"))
  ;[1 1 1] Audio Seeking
  (:`Pressed`
    (`self.seekAudio` (`self.Audio`) (`self.audioElapsedTime`) 5.0)))

(event `Key|Left`
  (params (Key :type "Key Structure"))
  ;[1 1 1] Audio Seeking
  (:`Pressed`
    (`self.seekAudio` (`self.Audio`) (`self.audioElapsedTime`) -5.0)))

(event `Key|SpaceBar`
  (params (Key :type "Key Structure"))
  (bind _audio (`self.Audio`))
  ;[1 1 1] Audio
  (:`Pressed`
    (if (`|EnumEquality` (`AudioComponent.GetPlayState` (`self.Audio`)) "Stopped")
      (`/Engine/EditorBlueprintResources/StandardMacros.DoOnce` false
        (:`Completed`
          (`AudioComponent.Play` (`self.Audio`) 0.0)))
      (else
        (`AudioComponent.SetPaused` _audio (not (`|EnumEquality` (`AudioComponent.GetPlayState` _audio) "Paused")))))))

(event `UpdateSongElapsed`
  (params (PlayingSoundWave :type "SoundWave Object Reference") (PlaybackPercent :type "Float (single-precision)"))
  (bind _debugaudio (`self.debugAudio`))
  (bind _returnvalue (`KismetMathLibrary.FMax` (- (`self.audioElapsedTime`) (`self.XR_Delay`))))
  ;[0.6439 0 1] Audio
  (bind _output_get (set `self.audioElapsedTime` (* (`SoundBase.Duration` PlayingSoundWave) PlaybackPercent)))
  (`KismetSystemLibrary.PrintString` (`KismetStringLibrary.Concat_StrStr` "Audio Elapsed: " (`KismetStringLibrary.Conv_DoubleToString` _output_get)) _debugaudio _debugaudio (struct :`G` 0.66 :`B` 1.0 :`A` 1.0) 10.0 "AudioElapsedTime")
  ;[0.644 0 1] Audio
  (if (not (`|EnumEquality` (`AudioComponent.GetPlayState` (`self.Audio`)) "Paused"))
    (for (_array_element _array_index) (`self.LoudnessAnalyzers`)
      (`KismetArrayLibrary.Array_Set` (`self.currentLoudnesses`) _array_index (`LoudnessNRT.GetNormalizedLoudnessAtTime` _array_element (`self.audioElapsedTime`))))
    (`self.UpdateAudioAnalysis` (`self.currentLoudnesses`) (`self.LoudnessAnalyzers`) (`self.Q_Analyzers`) _returnvalue (* _returnvalue (`self.audioDurationFraction`)))))

(fn `seekAudio`
  (params (Audio :type "AudioComponent Object Reference") (`Audio Current Time (S)` :type "Float (double-precision)") (`Seek Delta (S)` :type "Float (double-precision)"))
  (locals (isPaused :type Boolean))
  (bind _debugaudio (`self.debugAudio`))
  (bind _returnvalue (`KismetMathLibrary.FClamp` (+ `Audio Current Time (S)` `Seek Delta (S)`) 0.01 (`SoundBase.Duration` (`AudioComponent.Sound` Audio))))
  ;[1 1 1] If Currently playing, keep playing at advanced spot
  ; Else, seek forward/back, but immediately pause
  (if (`|EnumEquality` (`AudioComponent.GetPlayState` Audio) "Paused")
    (`AudioComponent.SetPaused` Audio false))
  (`AudioComponent.Play` Audio _returnvalue)
  (`KismetSystemLibrary.PrintString` (`KismetStringLibrary.Concat_StrStr` "New Seek Pos: " (`KismetStringLibrary.Conv_DoubleToString` _returnvalue)) _debugaudio _debugaudio (struct :`G` 0.66 :`B` 1.0 :`A` 1.0) 2.0 "debug seek")
  (return))

(fn `standardizeInput`
  (params (deviceName :type String) (controlID_ :type Integer) (velocity_ :type Integer) (eventType_ :type Integer))
  (returns (controlId :type Integer) (velocity :type Integer) (eventType :type Integer))
  (return controlID_ velocity_ eventType_))

(fn `UserConstructionScript`
  (set `self.audioDurationFraction` 0.0)
  ;[1 1 1] Comment
  (`KismetArrayLibrary.Array_Resize` (`self.currentLoudnesses`) (`KismetArrayLibrary.Array_Length` (`self.LoudnessAnalyzers`))))